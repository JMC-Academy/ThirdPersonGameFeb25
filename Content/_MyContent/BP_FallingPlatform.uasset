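; BP_FallingPlatform is a platform that vanishes after the third-person character stays on it past a time limit, then reappears after a respawn delay.
; Overlap events on Collision track the player and reset the timer, while Tick accumulates time and toggles the mesh's visibility and collision around a Delay.
; On entry a new dynamic material instance tints the mesh pink with reduced opacity, which is never reverted; debug prints show contact and elapsed time.
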(event `self.Collision.OnComponentBeginOverlap`
  (params (OverlappedComponent :type "PrimitiveComponent Object Reference") (OtherActor :type "Actor Object Reference") (OtherComp :type "PrimitiveComponent Object Reference") (OtherBodyIndex :type Integer) (bFromSweep :type Boolean) (SweepResult :type "HitResult Structure (by ref)"))
  (cast `/Game/ThirdPerson/Blueprints/BP_ThirdPersonCharacter` OtherActor)
  (`|ExecutionSequence`
    (:`then_0`
      (bind _returnvalue (`PrimitiveComponent.CreateDynamicMaterialInstance` (`self.SM_Platfrom`) 0 "/Game/_MyContent/MI_FallingPlatform.MI_FallingPlatform" "None"))
      (`MaterialInstanceDynamic.SetVectorParameterValue` _returnvalue "Colour" (struct :`R` 1.0 :`G` 0.254062 :`B` 0.700502 :`A` 1.0))
      (`MaterialInstanceDynamic.SetScalarParameterValue` _returnvalue "Opacity" 0.5))
    (:`then_1`
      (`KismetSystemLibrary.PrintString` "On Platform")
      (set `self.PlayerOnPlatform` true)
      (set `self.TimeOnPlatform` 0.0 :!label _label))))

(event `self.Collision.OnComponentEndOverlap`
  (params (OverlappedComponent :type "PrimitiveComponent Object Reference") (OtherActor :type "Actor Object Reference") (OtherComp :type "PrimitiveComponent Object Reference") (OtherBodyIndex :type Integer))
  (cast `/Game/ThirdPerson/Blueprints/BP_ThirdPersonCharacter` OtherActor)
  (set `self.PlayerOnPlatform` false)
  (goto _label))

(event `self.ReceiveTick`
  (params (DeltaSeconds :type "Float (single-precision)"))
  (if (`self.PlayerOnPlatform`)
    (set `self.TimeOnPlatform` (+ DeltaSeconds (`self.TimeOnPlatform`)))
    (`KismetSystemLibrary.PrintString` (`KismetStringLibrary.Conv_DoubleToString` (`self.TimeOnPlatform`)))
    (if (>= (`self.TimeOnPlatform`) (`self.TimeLimit`))
      (`SceneComponent.SetVisibility` (`self.SM_Platfrom`) false false)
      (`PrimitiveComponent.SetCollisionEnabled` (`self.SM_Platfrom`) "NoCollision")
      (`KismetSystemLibrary.Delay` (`self.RespawnDelay`))
      (`SceneComponent.SetVisibility` (`self.SM_Platfrom`) true false)
      (`PrimitiveComponent.SetCollisionEnabled` (`self.SM_Platfrom`) "QueryAndPhysics"))))

(fn `UserConstructionScript`)