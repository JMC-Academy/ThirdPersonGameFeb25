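; NPC actor that plays a timed sequence of dialogue lines when an actor tagged Player overlaps it.
; The overlap resets the line index, then a self-calling update event steps through the Dialogue array with a short delay between lines.
; Each line is written to CurrentDialogueText on the player's BP_ThirdPersonCharacter, which is cleared after the last line.
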(event `self.ReceiveActorBeginOverlap`
  (params (OtherActor :type "Actor Object Reference"))
  (if (`self.ActorHasTag` OtherActor "Player")
    (`self.ResetDialogue`)))

(event `ResetDialogue`
  (set `self.CurrDialogue` 0)
  (`self.UpdateDialogue`))

(event `UpdateDialogue`
  (bind _asbp_third_person_character (cast `/Game/ThirdPerson/Blueprints/BP_ThirdPersonCharacter` (`GameplayStatics.GetPlayerCharacter` 0)))
  (set `/Game/ThirdPerson/Blueprints/BP_ThirdPersonCharacter.CurrentDialogueText` (`|GetArrayItem` (`self.Dialogue`) (`self.CurrDialogue`)) _asbp_third_person_character)
  (set `self.CurrDialogue` (+ (`self.CurrDialogue`) 1))
  (`KismetSystemLibrary.Delay` 2.0)
  (if (!= (`self.CurrDialogue`) (`KismetArrayLibrary.Array_Length` (`self.Dialogue`)))
    (`self.UpdateDialogue`)
    (else
      (bind _asbp_third_person_character_2 (cast `/Game/ThirdPerson/Blueprints/BP_ThirdPersonCharacter` (`GameplayStatics.GetPlayerCharacter` 0)))
      (set `/Game/ThirdPerson/Blueprints/BP_ThirdPersonCharacter.CurrentDialogueText` "" _asbp_third_person_character_2))))

(fn `UserConstructionScript`)