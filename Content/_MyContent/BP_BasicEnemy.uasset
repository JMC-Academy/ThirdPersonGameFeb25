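; BP_BasicEnemy is a simple enemy that takes damage when the third-person player character overlaps it.
; Each overlap launches the player along LaunchDir and removes one point of the enemy's Health.
; When Health runs out, the DropLoot event spawns a BP_Coin at the enemy's transform and the enemy destroys itself.
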(event `self.ReceiveActorBeginOverlap`
  (params (OtherActor :type "Actor Object Reference"))
  (bind _asbp_third_person_character (cast `/Game/ThirdPerson/Blueprints/BP_ThirdPersonCharacter` OtherActor))
  (`Character.LaunchCharacter` _asbp_third_person_character (`self.LaunchDir`) false false)
  (set `self.Health` (- (`self.Health`) 1))
  (if (<= (`self.Health`) 0)
    (`self.DropLoot`)
    (`self.K2_DestroyActor`)))

(event `self.ReceiveHit`
  (params (MyComp :type "PrimitiveComponent Object Reference") (Other :type "Actor Object Reference") (OtherComp :type "PrimitiveComponent Object Reference") (bSelfMoved :type Boolean) (HitLocation :type "Vector Structure") (HitNormal :type "Vector Structure") (NormalImpulse :type "Vector Structure") (Hit :type "HitResult Structure (by ref)")))

(event `DropLoot`
  (`|SpawnActorFromClass` "/Game/_MyContent/BP_Coin.BP_Coin_C" (`self.GetTransform`) "Undefined" "MultiplyWithRoot" null null))

(fn `UserConstructionScript`)